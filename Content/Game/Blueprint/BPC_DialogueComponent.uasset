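; BPC_DialogueComponent is a dialogue component that reads dialogue lines from a data table.
; It looks up a row named after the current row number and caches it as the current dialogue row.
; Getters expose that row's long text and character, and a negative NewRow value marks the dialogue as finished.
; ReadNextRow is an empty stub, so advancing between rows is not implemented here.
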(fn GetCurrentDialogueRow
  (bind _returnvalue (Utilities|GetDataTableRow (Variables|Default|GetDialogueDataTable) (Utilities|String|StringToName (Utilities|String|ToString(Integer) (Variables|Default|GetCurrentRowNumber))))
    (:then
      (bind _output_get (Variables|Default|SetCurrentDialogueRow _returnvalue))
      (return _output_get))))

(fn GetDialogueLongfromCurrentRow
  (return (.DialogueLong (Utilities|Struct|BreakSt_DialogueRowDatas (Variables|Default|GetCurrentDialogueRow)))))

(fn GetCharacterfromRow
  (return (.Character (Utilities|Struct|BreakSt_DialogueRowDatas (Variables|Default|GetCurrentDialogueRow)))))

(fn IsDialogueFinished
  (return (< (.NewRow (Utilities|Struct|BreakSt_DialogueRowDatas (Variables|Default|GetCurrentDialogueRow))) 0)))

(fn ReadNextRow)